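; Player pawn for lane-based movement, with a coin counter and regenerating health.
; Left and right inputs step a clamped index through three preset Y positions and snap the root component there, keeping X and Z.
; BeginPlay starts in the middle lane, resets coins and runs a looping delay that adds HealthRegen whenever Health is not above 1.
; AddPoints increments the coin count by one.
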(event EventBeginPlay
  (Variables|Default|SetCurrentlyPosition 1)
  (Variables|Default|SetCoins 0)
  ;[1 0 0] Health Regen
  (Utilities|FlowControl|Delay 0.2 :!label _label)
  (if (> (Variables|Default|GetHealth) 1.0)
    (goto _label)
    (else
      (Variables|Default|SetHealth (+ (Variables|Default|GetHealth) (Variables|Default|GetHealthRegen)))
      (goto _label))))

(event Input|ActionEvents|InputActionMove_Right
  (params (Key :type Key%20Structure :default "None"))
  (bind _defaultsceneroot (Variables|Default|GetDefaultSceneRoot))
  (bind _returnvalue (Transformation|GetWorldLocation _defaultsceneroot))
  (:Pressed
    (Math|Integer|IncrementInt (Variables|Default|GetCurrentlyPosition)
      (:%20%20
        (Variables|Default|SetCurrentlyPosition (Math|Integer|Clamp(Integer) (Variables|Default|GetCurrentlyPosition) 0 2))
        (Transformation|SetWorldLocation _defaultsceneroot (Math|Vector|MakeVector (.x _returnvalue) (Utilities|Array|Get(acopy) (Variables|Default|GetPossiblyYPositions) (Variables|Default|GetCurrentlyPosition)) (.z _returnvalue)) false false)))))

(event Input|ActionEvents|InputActionMove_Left
  (params (Key :type Key%20Structure :default "None"))
  (bind _defaultsceneroot (Variables|Default|GetDefaultSceneRoot))
  (bind _returnvalue (Transformation|GetWorldLocation _defaultsceneroot))
  (:Pressed
    (Math|Integer|DecrementInt (Variables|Default|GetCurrentlyPosition)
      (:%20%20
        (Variables|Default|SetCurrentlyPosition (Math|Integer|Clamp(Integer) (Variables|Default|GetCurrentlyPosition) 0 2))
        (Transformation|SetWorldLocation _defaultsceneroot (Math|Vector|MakeVector (.x _returnvalue) (Utilities|Array|Get(acopy) (Variables|Default|GetPossiblyYPositions) (Variables|Default|GetCurrentlyPosition)) (.z _returnvalue)) false false)))))

(fn ConstructionScript)

(fn AddPoints
  (bind _result (Math|Integer|IncrementInt (Variables|Default|GetCoins))
    (:%20%20
      (Variables|Default|SetCoins _result))))