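; Boss-fight projectile that eases toward a stored player position on spawn and either damages the player or gets sent back at the boss.
; CanHurtBoss picks the variant: harmful shots get a different sphere material and reduce player health on overlap, without being destroyed here.
; Returnable shots reverse toward the boss's cube on player contact, calling LoseLife if they overlap the boss, and destroy themselves on hit or move completion.
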(event EventBeginPlay
  (if (Variables|Default|GetcanHurtBoss)
    _
    (else
      (Rendering|Material|SetMaterial (Variables|Default|GetSphere) 0 "/Game/StarterContent/Materials/M_Wood_Floor_Walnut_Polished.M_Wood_Floor_Walnut_Polished")))
  (Components|MoveComponentTo (Variables|Default|GetDefaultSceneRoot) (Variables|Default|GetPlayerPos) "0, 0, 0" true false 0.8 false))

(event Collision|EventActorBeginOverlap
  (params (OtherActor :type Actor%20Object%20Reference))
  (bind _returnvalue (Game|GetPlayerController 0))
  (bind _returnvalue_2 (Pawn|GetControlledPawn _returnvalue))
  (Utilities|FlowControl|Sequence
    (:then_0
      (if (== OtherActor _returnvalue_2)
        (if (Variables|Default|GetcanHurtBoss)
          (Variables|Default|SetisReturning true)
          (Components|MoveComponentTo (Variables|Default|GetDefaultSceneRoot) (Transformation|GetWorldLocation (Variables|/Game/Assets/Boss_BP.Boss_BP_C|GetCube (Variables|Default|GetBossReference))) "0, 0, 0" true false 0.8 false)
          (Actor|DestroyActor)
          (else
            (bind _aspawn_player_bp (Utilities|Casting|CastToPawnPlayer_BP _returnvalue_2))
            (Variables|/Game/Assets/PawnPlayer_BP.PawnPlayer_BP_C|SetHealth _aspawn_player_bp (- (Variables|/Game/Assets/PawnPlayer_BP.PawnPlayer_BP_C|GetHealth _aspawn_player_bp) 0.2))))))
    (:then_1
      (if (Variables|Default|GetisReturning)
        (if (== OtherActor (Variables|Default|GetBossReference))
          (Default|LoseLife (Variables|Default|GetBossReference))
          (Actor|DestroyActor))))))

(fn ConstructionScript)