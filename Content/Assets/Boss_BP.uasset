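; Boss actor that slides into position, fires projectiles at the player and returns in a repeating cycle after each defeat.
; Tick runs a delayed loop spawning BossProjectile_BP aimed at the player's X and a random Y from the player's position list.
; A random minority of projectiles can hurt the boss, and each receives a boss reference.
; When Life, decremented by LoseLife, runs out, the boss exits, resets, waits and re-enters.
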(event EventBeginPlay
  (bind _defaultsceneroot (Variables|Default|GetDefaultSceneRoot))
  (bind _returnvalue (Transformation|GetWorldLocation _defaultsceneroot))
  (bind _aspawn_player_bp (Utilities|Casting|CastToPawnPlayer_BP (Pawn|GetControlledPawn (Game|GetPlayerController 0))))
  (Variables|Default|SetPawnPlayerRef _aspawn_player_bp)
  (Variables|Default|SetMovimentationDone false)
  (Components|MoveComponentTo _defaultsceneroot (Math|Vector|MakeVector 8e+02 (.y _returnvalue) (.z _returnvalue)) "0, 0, 0" true true 3.0 false)
  (Variables|Default|SetMovimentationDone true)
  (Variables|Default|SetcanAttack true))

(event EventTick
  (params (DeltaSeconds :type Float%20%28single-precision%29))
  (bind _defaultsceneroot (Variables|Default|GetDefaultSceneRoot))
  (bind _pawnplayerref (Variables|Default|GetPawnPlayerRef))
  (bind _defaultsceneroot_2 (Variables|Default|GetDefaultSceneRoot))
  (bind _defaultsceneroot_3 (Variables|Default|GetDefaultSceneRoot))
  (bind _returnvalue (Transformation|GetWorldLocation _defaultsceneroot))
  (bind _returnvalue_2 (Transformation|GetWorldTransform _defaultsceneroot_3))
  (bind _returnvalue_3 (Transformation|GetWorldLocation _defaultsceneroot_2))
  (bind _possiblyypositions (Variables|/Game/Assets/PawnPlayer_BP.PawnPlayer_BP_C|GetPossiblyYPositions _pawnplayerref))
  (Utilities|FlowControl|Sequence
    (:then_1
      (if (Variables|Default|GetMovimentationDone)
        (Utilities|FlowControl|Delay 1.5 :!label _label)
        (bind _returnvalue_4 (Game|SpawnActorfromClass "/Game/Assets/BossProjectile_BP.BossProjectile_BP_C" (Math|Transform|MakeTransform (.location _returnvalue_2) (.rotation _returnvalue_2) "1,1,1") "Undefined" 0 (Math|Vector|MakeVector (.x (Transformation|GetWorldLocation (Variables|/Game/Assets/PawnPlayer_BP.PawnPlayer_BP_C|GetDefaultSceneRoot (Variables|Default|GetPawnPlayerRef)))) (Utilities|Array|Get(acopy) _possiblyypositions (Math|Random|RandomIntegerinRange 0 (- (Utilities|Array|Length _possiblyypositions) 1))) 0.0) (<= (Math|Random|RandomInteger 10) 2) 0))
        (Variables|/Game/Assets/BossProjectile_BP.BossProjectile_BP_C|SetBossReference _returnvalue_4 self)
        (if (Variables|Default|GetcanAttack)
          (goto _label))))
    (:then_2
      (if (<= (Variables|Default|GetLife) 0)
        (Variables|Default|SetcanAttack false)
        (if (Variables|Default|GetMovimentationDone)
          (Variables|Default|SetMovimentationDone false)
          (Components|MoveComponentTo _defaultsceneroot (Math|Vector|MakeVector 1.2e+04 (.y _returnvalue) (.z _returnvalue)) "0, 0, 0" false true 3.0 false)
          (Variables|Default|SetLife 5)
          (Transformation|SetWorldLocation (Variables|Default|GetDefaultSceneRoot) (Math|Vector|MakeVector -3e+03 0.0 (.z _returnvalue)) false true)
          (Utilities|FlowControl|Delay 1e+01)
          (Components|MoveComponentTo _defaultsceneroot_2 (Math|Vector|MakeVector 8e+02 (.y _returnvalue_3) (.z _returnvalue_3)) "0, 0, 0" true true 3.0 false)
          (Variables|Default|SetMovimentationDone true)
          (Variables|Default|SetcanAttack true))))))

(fn ConstructionScript)

(fn LoseLife
  (bind _result (Math|Integer|DecrementInt (Variables|Default|GetLife))
    (:%20%20
      (bind _output_get (Variables|Default|SetLife _result))
      (Development|PrintString (Utilities|String|ToString(Integer) _output_get)))))

(fn InitialMove)