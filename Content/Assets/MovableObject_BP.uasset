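; MovableObject_BP is an actor that scrolls along world negative X and removes itself once it travels far enough.
; Tick calls MoveObject, which shifts the root component by a fixed step each frame, unscaled by delta time, so speed depends on frame rate.
; After moving, it destroys the actor when its X position reaches a hardcoded lower limit.
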(event EventTick
  (params (DeltaSeconds :type Float%20%28single-precision%29))
  (CallFunction|MoveObject))

(fn ConstructionScript)

(fn MoveObject
  (bind _defaultsceneroot (Variables|Default|GetDefaultSceneRoot))
  (bind _defaultsceneroot_2 (Variables|Default|GetDefaultSceneRoot))
  (bind _returnvalue (Transformation|GetWorldLocation _defaultsceneroot_2))
  (Transformation|SetWorldLocation _defaultsceneroot_2 (Math|Vector|MakeVector (- (.x _returnvalue) 15.0) (.y _returnvalue) (.z _returnvalue)) false false)
  (Utilities|IsValid _defaultsceneroot
    (:Is%20Valid
      (if (<= (.x (Transformation|GetWorldLocation _defaultsceneroot)) -5e+03)
        (Actor|DestroyActor)))))